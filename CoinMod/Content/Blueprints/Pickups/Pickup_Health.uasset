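; Health pickup for a Pavlov game mode that adds health, armour and optionally a helmet to the interacting player.
; On the authority, it caches the first GameLogic_Coins actor after a short delay, and CanPickup only allows pickup once that reference is valid.
; CharacterInteract reads the player's status, clamps the new totals, keeps any existing helmet and applies them through SetPlayerVitality, reporting success or failure.
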(event `self.ReceiveBeginPlay`
  (`/Engine/EditorBlueprintResources/ActorMacros.Switch Has Authority`
    (:`Authority`
      (`KismetSystemLibrary.Delay` 1.5)
      (bind _outactors (`GameplayStatics.GetAllActorsOfClass` "/CoinMod/Blueprints/GameLogic_Coins.GameLogic_Coins_C"))
      (if (`KismetArrayLibrary.Array_IsValidIndex` _outactors)
        (set `self.GameLogic` (`|GetArrayItem` _outactors))))))

(fn `CanPickup`
  (params (Character :type "Character Object Reference"))
  (returns (CanPickup :type Boolean))
  (`self.GameLogic`
    (:`then`
      (return true))
    (:`else`
      (return false))))

(fn `CharacterInteract`
  (params (Character :type "Character Object Reference"))
  (returns (Successful :type Boolean))
  (`/Engine/EditorBlueprintResources/StandardMacros.IsValid` Character
    (:`Is Valid`
      (bind _playerstate (`Pawn.PlayerState` Character)
        (:`then`
          (bind (_playerstatus _bsucceeded) (`PavlovProxyStatics.GetPavlovPlayerStatus` _playerstate))
          (if _bsucceeded
            (bind (_playerstate_2 _controller _pawn _steamid _cash _score _teamid _health _armour _bhelmet) (break `PavlovPlayerStatus` _playerstatus))
            (`Pavlov_GameLogic.SetPlayerVitality` (`self.GameLogic`) _playerstate (`KismetMathLibrary.Clamp` (+ _health (`self.Health`)) 0 100) (`KismetMathLibrary.Clamp` (+ _armour (`self.Armour`)) 0 100) (select `bool` _bhelmet :`false` (`self.Helmet`) :`true` 1))
            (return true)
            (else
              _)))
        (:`else`
          _)))
    (:`Is Not Valid`
      _))
  (return false))

(fn `UserConstructionScript`
  (`parent.UserConstructionScript`))