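; Base pickup actor that characters collect by overlapping its static mesh, with the logic run only on network authority.
; CanPickup gates the overlap and CharacterInteract applies the pickup, both stubs returning true that appear intended for child overrides.
; A DoOnce prevents repeat collection and reopens if the interaction fails.
; Successful pickup, like ResetActor, sets a short lifespan to destroy the actor.
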(event `/CoinMod/Blueprints/Interfaces/BPI_Reset.ResetActor`
  (`self.SetLifeSpan` 0.25))

(event `self.StaticMesh.OnComponentBeginOverlap`
  (params (OverlappedComponent :type "PrimitiveComponent Object Reference") (OtherActor :type "Actor Object Reference") (OtherComp :type "PrimitiveComponent Object Reference") (OtherBodyIndex :type Integer) (bFromSweep :type Boolean) (SweepResult :type "HitResult Structure (by ref)"))
  (`/Engine/EditorBlueprintResources/ActorMacros.Switch Has Authority`
    (:`Authority`
      (bind _ascharacter (cast `Character` OtherActor))
      (if (`self.CanPickup` _ascharacter)
        (`/Engine/EditorBlueprintResources/StandardMacros.DoOnce` false :!label _label
          (:`Completed`
            (bind _successful (`self.CharacterInteract` _ascharacter))
            (if _successful
              (`self.SetLifeSpan` 0.25)
              (else
                (goto _label :!via `Reset`)))))))))

(fn `CanPickup`
  (params (Character :type "Character Object Reference"))
  (returns (CanPickup :type Boolean))
  (return true))

(fn `CharacterInteract`
  (params (Character :type "Character Object Reference"))
  (returns (Successful :type Boolean))
  (return true))

(fn `UserConstructionScript`)