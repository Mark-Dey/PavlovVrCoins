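; Networked coin pickup that credits its coin amount to the interacting character's player.
; The server allows pickup only after a short delay, while clients show the amount on a text render after their own delay and on each Coins RepNotify.
; SetCoins flushes net dormancy so changes replicate.
; Interaction adds the coins through the PlayerState's CMP_PlayerInfo component, which also plays the pickup sound, and reports success or failure.
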(event `self.ReceiveBeginPlay`
  (`/Engine/EditorBlueprintResources/ActorMacros.Switch Has Authority`
    (:`Authority`
      (`KismetSystemLibrary.Delay` 2.0)
      (set `self.CanPickupCoins` true))
    (:`Remote`
      (`KismetSystemLibrary.Delay` 1.5)
      (`TextRenderComponent.K2_SetText` (`self.TextRender`) (`KismetTextLibrary.Conv_IntToText` (`self.Coins`))))))

(fn `CanPickup`
  (params (Character :type "Character Object Reference"))
  (returns (CanPickup :type Boolean))
  (return (`self.CanPickupCoins`)))

(fn `CharacterInteract`
  (params (Character :type "Character Object Reference"))
  (returns (Successful :type Boolean))
  (`/Engine/EditorBlueprintResources/StandardMacros.IsValid` Character
    (:`Is Valid`
      (bind _playerstate (`Pawn.PlayerState` Character)
        (:`then`
          (bind _returnvalue (`self.GetComponentByClass` _playerstate "/CoinMod/Blueprints/CMPs/CMP_PlayerInfo.CMP_PlayerInfo_C"))
          (`/Engine/EditorBlueprintResources/StandardMacros.IsValid` _returnvalue
            (:`Is Valid`
              (`/CoinMod/Blueprints/CMPs/CMP_PlayerInfo.AddCoins` _returnvalue (`self.Coins`))
              (`/CoinMod/Blueprints/CMPs/CMP_PlayerInfo.PlaySound_Multi` _returnvalue "/CoinMod/Sounds/UI_CoinPickup_Test_1_Cue.UI_CoinPickup_Test_1_Cue")
              (return true))
            (:`Is Not Valid`
              _)))
        (:`else`
          _)))
    (:`Is Not Valid`
      _))
  (return false))

(fn `OnRep_Coins`
  (`TextRenderComponent.K2_SetText` (`self.TextRender`) (`KismetTextLibrary.Conv_IntToText` (`self.Coins`))))

(fn `SetCoins`
  (params (Coins :type Integer))
  (set `self.Coins` Coins)
  (`self.FlushNetDormancy`)
  (return))

(fn `UserConstructionScript`
  (`parent.UserConstructionScript`))