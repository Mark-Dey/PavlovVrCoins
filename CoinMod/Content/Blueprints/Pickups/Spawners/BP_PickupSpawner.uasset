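; Pickup spawner actor that keeps one pickup of a configurable class at its location.
; On the server, it starts a looping timer with a random interval shortly after BeginPlay, optionally spawning at once.
; Each tick of that timer spawns a replacement only when no valid pickup exists, then calls an empty OnPickupSpawned hook.
; ResetActor expires the current pickup after a short delay and restarts the timer.
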(event `/CoinMod/Blueprints/Interfaces/BPI_Reset.ResetActor`
  (`KismetSystemLibrary.Delay` 1.0)
  (bind _pickup (`self.Pickup`)
    (:`then`
      (`self.SetLifeSpan` _pickup 0.25)
      (set `self.Pickup` null))
    (:`else`
      _))
  (`self.Start SpawnTimer`))

(event `self.ReceiveBeginPlay`
  (`/Engine/EditorBlueprintResources/ActorMacros.Switch Has Authority`
    (:`Authority`
      (`KismetSystemLibrary.Delay` 2.0)
      (`self.Start SpawnTimer`))))

(event `Start SpawnTimer`
  (bind _returnvalue (`KismetSystemLibrary.K2_SetTimerDelegate` (delegate `SpawnItem`) (`KismetMathLibrary.RandomFloatInRange` (`self.SpawnTimerMin`) (`self.SpawnTimerMax`)) true))
  (set `self.SpawnerTimerHandle` _returnvalue)
  (if (`self.SpawnWhenTimerStarts`)
    (`self.SpawnItem`)))

(event `SpawnItem`
  (bind (_returnvalue_location _returnvalue_rotation) (`KismetMathLibrary.BreakTransform` (`self.GetTransform`)))
  (bind _pickupclass (`self.PickupClass`))
  (`self.Pickup`
    (:`then`)
    (:`else`
      (if (`KismetSystemLibrary.IsValidClass` _pickupclass)
        (bind _returnvalue (`|SpawnActorFromClass` _pickupclass (`KismetMathLibrary.MakeTransform` _returnvalue_location _returnvalue_rotation) "AdjustIfPossibleButAlwaysSpawn" "OverrideRootScale" null null))
        (bind _asbp_pickup (cast `/CoinMod/Blueprints/Pickups/BP_Pickup` _returnvalue))
        (bind _output_get (set `self.Pickup` _asbp_pickup))
        (`self.OnPickupSpawned` _output_get)))))

(fn `OnPickupSpawned`
  (params (Pickup :type "/CoinMod/Blueprints/Pickups/BP_Pickup Object Reference")))

(fn `UserConstructionScript`)