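; Player info component for a Pavlov game mode, expected on a PlayerState, tracking pawn, coins, team, lives, walk speed and low gravity.
; Server init hands movement settings to a client event, while OnRep functions reapply speed and gravity; timed boosts revert to a hard-coded default speed.
; Coins drive score by sending GameLogic the difference from the current Pavlov score.
; Coin gains count only during started rounds and trigger a winner check.
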(event `Reset Walk Speed`
  (params (Time :type "Float (double-precision)"))
  (`KismetSystemLibrary.K2_SetTimerDelegate` (delegate `SetWalkSpeedDefault`) Time))

(event `SetWalkSpeedDefault`
  (set `self.WalkSpeed` 350.0))

(event `InitPlayerInfo_Client`
  (params (Pawn :type "Pawn Object Reference") (WalkSpeed :type "Float (double-precision)") (LowGrav :type Boolean))
  (`/Engine/EditorBlueprintResources/StandardMacros.IsValid` Pawn
    (:`Is Valid`
      (bind _ascharacter_movement_component (cast `CharacterMovementComponent` (`Pawn.GetMovementComponent` Pawn)))
      (set `CharacterMovementComponent.MaxWalkSpeed` WalkSpeed _ascharacter_movement_component)
      (set `CharacterMovementComponent.GravityScale` (select `bool` LowGrav :`false` 1.0 :`true` 0.35 :!type "Float (single-precision)") _ascharacter_movement_component))))

(event `PlaySound_Multi`
  (params (Sound :type "SoundBase Object Reference"))
  (bind _pawn (`self.Pawn`))
  (if (and (`KismetSystemLibrary.IsValid` Sound) (`KismetSystemLibrary.IsValid` _pawn))
    (`GameplayStatics.PlaySoundAtLocation` Sound (`Actor.K2_GetActorLocation` _pawn) (struct) 1.0 1.0 0.0 null null null)))

(fn `AddCoins`
  (params (CoinsToAdd :type Integer))
  (returns (Current :type Integer))
  (bind _gamelogic (`self.GameLogic`)
    (:`then`
      (if (`|EnumEquality` (`Pavlov_GameLogic.GetRoundState` _gamelogic) "Started")
        (set `self.Coins` (`KismetMathLibrary.Clamp` (+ (`self.Coins`) CoinsToAdd) 0 500000))
        (`self.SetPlayerScore`)
        (`/CoinMod/Blueprints/GameLogic_Coins.CheckIfWinner` (`self.GameLogic`) self)))
    (:`else`
      _))
  (return (`self.Coins`)))

(fn `BoostWalkSpeed`
  (params (WalkSpeed :type "Float (double-precision)") (Duration :type "Float (double-precision)"))
  (set `self.WalkSpeed` WalkSpeed)
  (`self.Reset Walk Speed` Duration))

(fn `InitPlayerInfo_Server`
  (params (Pawn :type "Pawn Object Reference") (WalkSpeed :type "Float (double-precision)" :default 350.0) (Coins :type Integer) (TeamID :type Integer) (LowGrav :type Boolean) (GameLogic :type "/CoinMod/Blueprints/GameLogic_Coins Object Reference") (Lives :type Integer))
  (bind _output_get (set `self.Pawn` Pawn))
  (bind _output_get_2 (set `self.WalkSpeed` WalkSpeed))
  (set `self.Coins` Coins)
  (set `self.TeamID` TeamID)
  (set `self.LowGrav` LowGrav)
  (set `self.GameLogic` GameLogic)
  (set `self.Lives` Lives)
  (`self.InitPlayerInfo_Client` _output_get _output_get_2 (`self.LowGrav`))
  (`self.SetPlayerScore`)
  (`/CoinMod/Blueprints/GameLogic_Coins.SetTeamScore` (`self.GameLogic`) (`self.TeamID`)))

(fn `OnRep_LowGrav`
  (bind _pawn (`self.Pawn`)
    (:`then`
      (bind _ascharacter_movement_component (cast `CharacterMovementComponent` (`Pawn.GetMovementComponent` _pawn)))
      (set `CharacterMovementComponent.GravityScale` (select `bool` (`self.LowGrav`) :`false` 1.0 :`true` 0.35 :!type "Float (single-precision)") _ascharacter_movement_component))
    (:`else`)))

(fn `OnRep_WalkSpeed`
  (bind _pawn (`self.Pawn`)
    (:`then`
      (bind _ascharacter_movement_component (cast `CharacterMovementComponent` (`Pawn.GetMovementComponent` _pawn)))
      (set `CharacterMovementComponent.MaxWalkSpeed` (`self.WalkSpeed`) _ascharacter_movement_component))
    (:`else`)))

(fn `ResetCoins`
  (params (Coins :type Integer))
  (set `self.Coins` Coins)
  (`self.SetPlayerScore`)
  (bind _gamelogic (`self.GameLogic`)
    (:`then`
      (if (not (`/CoinMod/Blueprints/GameLogic_Coins.NoTeams` _gamelogic))
        (`/CoinMod/Blueprints/GameLogic_Coins.SetTeamScore` _gamelogic (`self.TeamID`))))
    (:`else`
      _))
  (return))

(fn `SetPlayerScore`
  (locals (L_Score :type Integer))
  (bind _returnvalue (`self.GetOwner`))
  (`/Engine/EditorBlueprintResources/StandardMacros.IsValid` _returnvalue
    (:`Is Valid`
      (bind _asplayer_state (cast `PlayerState` _returnvalue)
        (:`then`
          (bind (_playerstatus _bsucceeded) (`PavlovProxyStatics.GetPavlovPlayerStatus` _asplayer_state))
          (if _bsucceeded
            (bind (_playerstate _controller _pawn _steamid _cash _score) (break `PavlovPlayerStatus` _playerstatus))
            (set `local.L_Score` _score)
            (bind _gamelogic (`self.GameLogic`)
              (:`then`
                (`Pavlov_GameLogic.IncrementPlayerScore` _gamelogic _playerstate (- (`self.Coins`) (`local.L_Score`))))
              (:`else`
                _))
            (return)
            (else
              _)))
        (:`CastFailed`
          _)))
    (:`Is Not Valid`
      _))
  (return))