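; Jump pad level actor that launches characters who overlap it.
; The construction script pitches an Arrow component by the Angle variable, so its forward vector sets the launch direction.
; CharacterOverlapped launches the character along that vector scaled by Boost, overriding existing horizontal and vertical velocity.
; The launch is wired only to the Remote branch of the authority switch, so it runs only without authority.
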(event `self.CharacterOverlapped`
  (params (Character :type "Character Object Reference"))
  (`/Engine/EditorBlueprintResources/ActorMacros.Switch Has Authority`
    (:`Remote`
      (`Character.LaunchCharacter` Character (* (`SceneComponent.GetForwardVector` (`self.Arrow`)) (`self.Boost`)) true true))))

(fn `UserConstructionScript`
  (`SceneComponent.K2_SetRelativeRotation` (`self.Arrow`) (`KismetMathLibrary.MakeRotator` 0.0 (`self.Angle`)) false false)
  (`parent.UserConstructionScript`))