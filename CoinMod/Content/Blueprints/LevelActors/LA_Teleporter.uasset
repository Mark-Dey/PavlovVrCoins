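; LA_Teleporter is a level actor that teleports an overlapping character to the location and rotation of its Capsule component.
; The CharacterOverlapped event does the work on the server only, behind an authority check, using the capsule's world transform as the destination.
; The graph has no other active logic, and the overlap detection that raises the event is not defined in it.
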(event `self.CharacterOverlapped`
  (params (Character :type "Character Object Reference"))
  (bind (_returnvalue_location _returnvalue_rotation) (`KismetMathLibrary.BreakTransform` (`SceneComponent.K2_GetComponentToWorld` (`self.Capsule`))))
  (`/Engine/EditorBlueprintResources/ActorMacros.Switch Has Authority`
    (:`Authority`
      (`self.K2_TeleportTo` Character _returnvalue_location _returnvalue_rotation))))

(fn `UserConstructionScript`
  (`parent.UserConstructionScript`))