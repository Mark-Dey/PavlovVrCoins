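; LA_SpeedBoost is a level actor that temporarily boosts the walk speed of a character that overlaps it.
; Its CharacterOverlapped event runs only on authority and looks up the CMP_PlayerInfo component on the character's PlayerState.
; When both are valid, it passes BoostSpeed and BoostDuration to that component's BoostWalkSpeed, which handles the boost.
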(event `self.CharacterOverlapped`
  (params (Character :type "Character Object Reference"))
  (`/Engine/EditorBlueprintResources/ActorMacros.Switch Has Authority`
    (:`Authority`
      (bind _playerstate (`Pawn.PlayerState` Character)
        (:`then`
          (bind _returnvalue (`self.GetComponentByClass` _playerstate "/CoinMod/Blueprints/CMPs/CMP_PlayerInfo.CMP_PlayerInfo_C"))
          (`/Engine/EditorBlueprintResources/StandardMacros.IsValid` _returnvalue
            (:`Is Valid`
              (`/CoinMod/Blueprints/CMPs/CMP_PlayerInfo.BoostWalkSpeed` _returnvalue (`self.BoostSpeed`) (`self.BoostDuration`)))))
        (:`else`)))))

(fn `UserConstructionScript`
  (`parent.UserConstructionScript`))