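; Level actor that marks a buy zone, letting players inside it buy through the coin game logic.
; On the server it caches the first GameLogic_Coins actor shortly after BeginPlay.
; CharacterOverlapped enables buying for that player's PlayerState with a long duration and wide range.
; Leaving the Box calls the same function with a very short duration and range, so buying expires almost immediately.
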(event `self.ReceiveBeginPlay`
  (`parent.ReceiveBeginPlay`)
  (`/Engine/EditorBlueprintResources/ActorMacros.Switch Has Authority`
    (:`Authority`
      (`KismetSystemLibrary.Delay` 1.5)
      (bind _outactors (`GameplayStatics.GetAllActorsOfClass` "/CoinMod/Blueprints/GameLogic_Coins.GameLogic_Coins_C"))
      (if (`KismetArrayLibrary.Array_IsValidIndex` _outactors)
        (set `self.GameLogic` (`|GetArrayItem` _outactors))))))

(event `self.CharacterOverlapped`
  (params (Character :type "Character Object Reference"))
  (`/Engine/EditorBlueprintResources/ActorMacros.Switch Has Authority`
    (:`Authority`
      (bind _playerstate (`Pawn.PlayerState` Character)
        (:`then`
          (bind _gamelogic (`self.GameLogic`)
            (:`then`
              (`Pavlov_GameLogic.SetPlayerBuyingEnabled` _gamelogic _playerstate 60.0 1000.0))
            (:`else`)))
        (:`else`)))))

(event `self.Box.OnComponentEndOverlap`
  (params (OverlappedComponent :type "PrimitiveComponent Object Reference") (OtherActor :type "Actor Object Reference") (OtherComp :type "PrimitiveComponent Object Reference") (OtherBodyIndex :type Integer))
  (`/Engine/EditorBlueprintResources/ActorMacros.Switch Has Authority`
    (:`Authority`
      (bind _ascharacter (cast `Character` OtherActor))
      (bind _playerstate (`Pawn.PlayerState` _ascharacter)
        (:`then`
          (bind _gamelogic (`self.GameLogic`)
            (:`then`
              (`Pavlov_GameLogic.SetPlayerBuyingEnabled` _gamelogic _playerstate 0.5 10.0))
            (:`else`)))
        (:`else`)))))

(fn `UserConstructionScript`
  (`parent.UserConstructionScript`))