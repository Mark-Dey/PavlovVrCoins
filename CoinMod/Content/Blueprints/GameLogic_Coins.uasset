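; Pavlov game-mode logic for a coin-collecting match, randomly set to free-for-all or teams at init.
; Players spawn with coins; deaths pass them to a living killer or drop a ground-traced pickup.
; CheckIfWinner tests player or living-team totals against targets, updating team scores and BP_Winner displays.
; Authority timers respawn dead players and flag the last round after an hour; round end kills survivors and resets actors.
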(event `self.ReceiveBeginPlay`
  (`/Engine/EditorBlueprintResources/ActorMacros.Switch Has Authority`
    (:`Authority`
      (`KismetSystemLibrary.Delay` 1.0)
      (`self.StartLastRoundTimer`)
      (`self.StartRespawnTimer`)
      (`self.SetFallDamage` false))))

(event `StartLastRoundTimer`
  (`KismetSystemLibrary.K2_SetTimerDelegate` (delegate `SetLastRound`) 3600.0))

(event `StartRespawnTimer`
  (`KismetSystemLibrary.K2_SetTimerDelegate` (delegate `RespawnDeadPlayers`) 1.0 true))

(event `SetLastRound`
  (set `self.LastRound` true))

(event `RespawnDeadPlayers`
  (if (`|EnumEquality` (`self.GetRoundState`) "Started")
    (for _array_element (`self.GetPlayer`)
      (bind (_playerstatus _bsucceeded) (`PavlovProxyStatics.GetPavlovPlayerStatus` _array_element))
      (if _bsucceeded
        (bind (_playerstate _controller _pawn _steamid _cash _score _teamid _health _armour _bhelmet _bdead _bcanbuy _bcrouching _bgagged _brighthanded _deadtime) (break `PavlovPlayerStatus` _playerstatus))
        (if (and _bdead (>= _deadtime 5.0))
          (`/Engine/EditorBlueprintResources/StandardMacros.IsValid` _controller
            (:`Is Valid`
              (bind _transform (`self.GetSpawnTransform` _controller))
              (`self.Spawn` _controller _transform))))))))

(event `self.OnPlayerKilled`
  (params (PlayerStatus :type "PavlovPlayerStatus Structure (by ref)") (Killer :type "PlayerState Object Reference"))
  (`self.PlayerKilled` PlayerStatus Killer))

(event `self.OnPlayerSpawned`
  (params (PlayerStatus :type "PavlovPlayerStatus Structure (by ref)"))
  (`self.PlayerSpawned` PlayerStatus))

(event `self.OnCustomGameModeInit`
  (set `self.NoTeams` (`KismetMathLibrary.RandomBool`))
  (`self.SetGameModeProperties` (make `PavlovGameModeProperties` (`self.NoTeams`) false true 16000 300 3300 false false 5.0 false false 30 10 true true (select `bool` (`self.NoTeams`) :`false` 600 :`true` 420))))

(event `self.OnRoundBegin`
  (`KismetSystemLibrary.Delay` 1.0)
  (`self.SetRoundState` "StandBy")
  (`self.PostRoundCleanUp`)
  (`self.InitScoreboards`)
  (`KismetSystemLibrary.Delay` 1.0)
  (`self.SetRoundState` "Started"))

(event `self.OnRoundEnd`
  (`KismetSystemLibrary.Delay` 4.0)
  (for _array_element (`self.GetPlayer`)
    (bind (_playerstatus _bsucceeded) (`PavlovProxyStatics.GetPavlovPlayerStatus` _array_element))
    (if _bsucceeded
      (bind (_playerstate _controller _pawn _steamid _cash _score _teamid _health _armour _bhelmet _bdead) (break `PavlovPlayerStatus` _playerstatus))
      (if (and (`KismetSystemLibrary.IsValid` _pawn) (not _bdead))
        (`GameplayStatics.ApplyDamage` _pawn 1000.0)
        (`self.IncrementPlayerScore` _playerstate (* _score -1)))))
  (`KismetSystemLibrary.Delay` 2.0)
  (`self.ResetTeamScore`)
  (`self.ResetActors`)
  (`KismetSystemLibrary.Delay` 1.0)
  (if (`self.LastRound`)
    (bind _asgame_mode (cast `GameMode` (`GameplayStatics.GetGameMode`)))
    (`GameMode.EndMatch` _asgame_mode)
    (else
      (`self.SetRoundState` "Starting"))))

(event `DeclareWinner`
  (params (TeamID :type Integer) (PlayerWin :type String))
  (`/Engine/EditorBlueprintResources/StandardMacros.DoOnce` false :!label _label
    (:`Completed`
      (`self.SetRoundState` "Ended")
      (`self.SetWinnerInfo` TeamID PlayerWin)
      (`KismetSystemLibrary.Delay` 5.0)
      (goto _label :!via `Reset`))))

(event `self.OnPlayerLeftServer`
  (params (PlayerStatus :type "PavlovPlayerStatus Structure (by ref)"))
  (`self.PlayerLeftServer` PlayerStatus))

(fn `CheckIfWinner`
  (params (PlayerInfoCMP :type "/CoinMod/Blueprints/CMPs/CMP_PlayerInfo Object Reference"))
  (locals (L_PlayerName :type String :default "None") (L_TeamID :type Integer :default 0))
  (if (`|EnumEquality` (`self.GetRoundState`) "Started")
    (bind _playerinfocmp (`local.PlayerInfoCMP`)
      (:`then`
        (if (`self.NoTeams`)
          (bind _asplayer_state (cast `PlayerState` (`ActorComponent.GetOwner` _playerinfocmp))
            (:`then`
              (set `local.L_PlayerName` (`PlayerState.PlayerName` _asplayer_state)))
            (:`CastFailed`
              _))
          (if (>= (`/CoinMod/Blueprints/CMPs/CMP_PlayerInfo.Coins` (`local.PlayerInfoCMP`)) (`self.CoinsToWinFFA`))
            (`self.DeclareWinner` -1 (`local.L_PlayerName`)))
          (else
            (bind _output_get (set `local.L_TeamID` (`/CoinMod/Blueprints/CMPs/CMP_PlayerInfo.TeamID` (`local.PlayerInfoCMP`))))
            (bind _winner (`self.SetTeamScore` _output_get))
            (if _winner
              (`self.DeclareWinner` (`local.L_TeamID`))))))
      (:`else`))))

(fn `GetPlayer`
  (returns (PlayerArray :type "Array of PlayerState Object Reference"))
  (return (`GameStateBase.PlayerArray` (`GameplayStatics.GetGameState`))))

(fn `GetTeamCoins`
  (params (TeamID :type Integer))
  (returns (Winner :type Boolean) (Coins :type Integer))
  (locals (L_PlayerInfo :type "/CoinMod/Blueprints/CMPs/CMP_PlayerInfo Object Reference") (L_Coins :type Integer :default 0) (L_Winner :type Boolean))
  (for _array_element (`self.GetPlayer`)
    (bind (_playerstatus _bsucceeded) (`PavlovProxyStatics.GetPavlovPlayerStatus` _array_element))
    (if _bsucceeded
      (bind (_playerstate _controller _pawn _steamid _cash _score _teamid _health _armour _bhelmet _bdead) (break `PavlovPlayerStatus` _playerstatus))
      (bind _returnvalue (`self.GetComponentByClass` _playerstate "/CoinMod/Blueprints/CMPs/CMP_PlayerInfo.CMP_PlayerInfo_C"))
      (if (and (`KismetSystemLibrary.IsValid` _returnvalue) (== _teamid (`local.TeamID`)) (not _bdead))
        (bind _output_get (set `local.L_PlayerInfo` _returnvalue))
        (set `local.L_Coins` (+ (`/CoinMod/Blueprints/CMPs/CMP_PlayerInfo.Coins` _output_get) (`local.L_Coins`)))
        (if (>= (`local.L_Coins`) (`self.CoinsToWinTDM`))
          (set `local.L_Winner` true)
          (break)))))
  (return (`local.L_Winner`) (`local.L_Coins`)))

(fn `InitScoreboards`
  (bind _noteams (`self.NoTeams`))
  (bind _outactors (`GameplayStatics.GetAllActorsOfClass` "/CoinMod/Widgets/BP_Winner.BP_Winner_C"))
  (for _array_element _outactors
    (`/CoinMod/Widgets/BP_Winner.SetWinner` _array_element "None")
    (`/CoinMod/Widgets/BP_Winner.InitRoundInfo` _array_element (select `bool` _noteams :`false` (`self.CoinsToWinTDM`) :`true` (`self.CoinsToWinFFA`)) _noteams))
  (return))

(fn `PlayerKilled`
  (params (PlayerStatus :type "PavlovPlayerStatus Structure (by ref)") (Killer :type "PlayerState Object Reference"))
  (locals (L_KilledPlayerState :type "PlayerState Object Reference") (L_Coins :type Integer :default 0) (L_PlayerInfo :type "/CoinMod/Blueprints/CMPs/CMP_PlayerInfo Object Reference") (L_KillerPlayerInfo :type "/CoinMod/Blueprints/CMPs/CMP_PlayerInfo Object Reference") (L_SpawnTransform :type "Transform Structure"))
  (bind _killer (`local.Killer`))
  (bind (_playerstate _controller _pawn _steamid) (break `PavlovPlayerStatus` (`local.PlayerStatus`)))
  (bind _returnvalue (`self.K2_GetActorLocation` _pawn))
  (if (`|EnumEquality` (`self.GetRoundState`) "Started")
    (bind _output_get (set `local.L_KilledPlayerState` (`.PlayerState` (break `PavlovPlayerStatus` (`local.PlayerStatus`)))))
    (bind _returnvalue_2 (`self.GetComponentByClass` _output_get "/CoinMod/Blueprints/CMPs/CMP_PlayerInfo.CMP_PlayerInfo_C"))
    (`/Engine/EditorBlueprintResources/StandardMacros.IsValid` _returnvalue_2
      (:`Is Valid`
        (bind _output_get_2 (set `local.L_PlayerInfo` _returnvalue_2))
        (set `local.L_Coins` (`/CoinMod/Blueprints/CMPs/CMP_PlayerInfo.Coins` _returnvalue_2))
        (`/CoinMod/Blueprints/CMPs/CMP_PlayerInfo.ResetCoins` _output_get_2 0)
        (`/Engine/EditorBlueprintResources/StandardMacros.IsValid` _killer
          (:`Is Valid`
            (if (not (== _killer (`local.L_KilledPlayerState`)))
              (bind (_playerstatus _bsucceeded) (`PavlovProxyStatics.GetPavlovPlayerStatus` (`local.Killer`)))
              (if _bsucceeded
                (bind (_playerstate_2 _controller_2 _pawn_2 _steamid_2 _cash _score _teamid _health _armour _bhelmet _bdead) (break `PavlovPlayerStatus` _playerstatus))
                (bind _returnvalue_3 (`self.GetComponentByClass` _playerstate_2 "/CoinMod/Blueprints/CMPs/CMP_PlayerInfo.CMP_PlayerInfo_C"))
                (if (and (`KismetSystemLibrary.IsValid` _returnvalue_3) (not _bdead))
                  (bind _output_get_3 (set `local.L_KillerPlayerInfo` _returnvalue_3))
                  (`/CoinMod/Blueprints/CMPs/CMP_PlayerInfo.AddCoins` _output_get_3 (`local.L_Coins`))
                  (return)
                  (else
                    _)))))
          (:`Is Not Valid`
            _))
        (`/Engine/EditorBlueprintResources/StandardMacros.IsValid` _pawn
          (:`Is Valid`
            (bind (_outhit _returnvalue_4) (`KismetSystemLibrary.LineTraceSingle` _returnvalue (- _returnvalue (0.0 0.0 500.0)) "TraceTypeQuery1" false (`|MakeArray` _pawn :!type "Actor Object Reference")))
            (if _returnvalue_4
              (set `local.L_SpawnTransform` (`KismetMathLibrary.Conv_VectorToTransform` (`.Location` (`GameplayStatics.BreakHitResult` _outhit))))
              (else
                (set `local.L_SpawnTransform` (`KismetMathLibrary.Conv_VectorToTransform` _returnvalue))))
            (bind _returnvalue_5 (`|SpawnActorFromClass` "/CoinMod/Blueprints/Pickups/Pickup_Coins.Pickup_Coins_C" (`local.L_SpawnTransform`) "AdjustIfPossibleButAlwaysSpawn" "OverrideRootScale" null null))
            (`/CoinMod/Blueprints/Pickups/Pickup_Coins.SetCoins` _returnvalue_5 (`local.L_Coins`))
            (return))
          (:`Is Not Valid`
            (`HealthSnapshotBlueprintLibrary.LogPerformanceSnapshot` (`KismetStringLibrary.Concat_StrStr` _steamid " Pawn not valid cant spawn coins at their location"))
            (return))))
      (:`Is Not Valid`
        _)))
  (return))

(fn `PlayerLeftServer`
  (params (PlayerStatus :type "PavlovPlayerStatus Structure (by ref)"))
  (bind _playerstate (break `PavlovPlayerStatus` PlayerStatus))
  (`/Engine/EditorBlueprintResources/StandardMacros.IsValid` _playerstate
    (:`Is Valid`
      (`/CoinMod/Blueprints/CMPs/CMP_PlayerInfo.ResetCoins` (`self.GetComponentByClass` _playerstate "/CoinMod/Blueprints/CMPs/CMP_PlayerInfo.CMP_PlayerInfo_C") 0))))

(fn `PlayerSpawned`
  (params (PlayerStatus :type "PavlovPlayerStatus Structure (by ref)"))
  (locals (L_PlayerState :type "PlayerState Object Reference") (L_PlayerInfo :type "/CoinMod/Blueprints/CMPs/CMP_PlayerInfo Object Reference") (L_Pawn :type "Pawn Object Reference"))
  (bind (_playerstate _controller _pawn _steamid _cash _score _teamid) (break `PavlovPlayerStatus` PlayerStatus))
  (bind _l_playerstate (`local.L_PlayerState`))
  (bind _returnvalue (`self.GetComponentByClass` (`local.L_PlayerState`) "/CoinMod/Blueprints/CMPs/CMP_PlayerInfo.CMP_PlayerInfo_C"))
  (set `local.L_PlayerState` _playerstate)
  (set `local.L_Pawn` _pawn)
  (`/Engine/EditorBlueprintResources/StandardMacros.IsValid` _returnvalue
    (:`Is Valid`
      (bind _output_get (set `local.L_PlayerInfo` _returnvalue))
      (`/CoinMod/Blueprints/CMPs/CMP_PlayerInfo.InitPlayerInfo_Server` (`local.L_PlayerInfo`) (`local.L_Pawn`) 350.0 5 _teamid true self (- (`/CoinMod/Blueprints/CMPs/CMP_PlayerInfo.Lives` _output_get) 1)))
    (:`Is Not Valid`
      (bind _returnvalue_2 (`AddComponent|NODE_AddCMP_PlayerInfo-0` :`self` (`local.L_PlayerState`)))
      (set `local.L_PlayerInfo` _returnvalue_2)
      (`/CoinMod/Blueprints/CMPs/CMP_PlayerInfo.InitPlayerInfo_Server` (`local.L_PlayerInfo`) (`local.L_Pawn`) 350.0 5 _teamid true self 5)))
  (`self.SetPlayerVitality` _l_playerstate 100 100 1)
  (`self.SetPlayerBuyingEnabled` _l_playerstate 0.5 10.0)
  (`self.SpawnItem` (make `PavlovItemSpawnParams` "de" (`local.L_PlayerState`)))
  (return))

(fn `ResetActors`
  (bind _outactors (`GameplayStatics.GetAllActorsWithInterface` "/CoinMod/Blueprints/Interfaces/BPI_Reset.BPI_Reset_C"))
  (for _array_element _outactors
    (message `/CoinMod/Blueprints/Interfaces/BPI_Reset.ResetActor` _array_element))
  (return))

(fn `ResetTeamScore`
  (if (not (`self.NoTeams`))
    (bind _score (`PavlovProxyStatics.GetTeamScore` 0))
    (`self.IncrementTeamScore` 0 (* _score -1))
    (bind _score_2 (`PavlovProxyStatics.GetTeamScore` 1))
    (`self.IncrementTeamScore` 1 (* _score_2 -1)))
  (return))

(fn `SetTeamScore`
  (params (TeamID :type Integer))
  (returns (Winner :type Boolean))
  (locals (L_Winner :type Boolean :default false) (L_Coins :type Integer :default 0))
  (bind (_winner _coins) (`self.GetTeamCoins` TeamID))
  (set `local.L_Winner` _winner)
  (set `local.L_Coins` _coins)
  (bind _score (`PavlovProxyStatics.GetTeamScore` (`local.TeamID`)))
  (`self.IncrementTeamScore` (`local.TeamID`) (- (`local.L_Coins`) _score))
  (return (`local.L_Winner`)))

(fn `SetWinnerInfo`
  (params (TeamID :type Integer) (PlayerWinner :type String))
  (bind _outactors (`GameplayStatics.GetAllActorsOfClass` "/CoinMod/Widgets/BP_Winner.BP_Winner_C"))
  (for _array_element _outactors
    (`/CoinMod/Widgets/BP_Winner.SetWinner` _array_element (select `bool` (`self.NoTeams`) :`false` (select `int` (`local.TeamID`) :`0` "Blue Team" :`1` "Red Team" :!type "Text") :`true` (`KismetTextLibrary.Conv_StringToText` (`local.PlayerWinner`))))))

(fn `UserConstructionScript`)